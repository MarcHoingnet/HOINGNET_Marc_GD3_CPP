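; BP_Cell_Recul is a setback cell for a board game that moves a player's pawn backward.
; Its Action override calls the parent, reads the player's current cell number from the game instance and subtracts NbrDeCaseEnMoins.
; The game mode's MovePawn then sends the pawn to that cell, followed by a fixed "-1" debug print.
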(event EventBeginPlay
  (|CallParentFunction) ; This node is disabled and will not be called.\nDrag off pins to build functionality.
)

(event Collision|EventActorBeginOverlap
  (params (OtherActor :type Actor%20Object%20Reference))
  (|CallParentFunction OtherActor) ; This node is disabled and will not be called.\nDrag off pins to build functionality.
)

(event EventTick
  (params (DeltaSeconds :type Float%20%28single-precision%29))
  (|CallParentFunction DeltaSeconds) ; This node is disabled and will not be called.\nDrag off pins to build functionality.
)

(fn ConstructionScript
  (|CallParentFunction))

(fn Action
  (params (PlayerID :type Integer))
  (|CallParentFunction PlayerID)
  (bind _playercellnumber (Default|GetPlayerCellNumberbyPlayerID (Variables|Default|GetAs%20BP%20Game%20Instance) PlayerID))
  (Default|MovePawn (Variables|Default|GetAs%20BP%20Game%20Mode) (- _playercellnumber (Variables|Default|GetNbrDeCaseEnMoins)) PlayerID)
  (Development|PrintString "-1"))