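; BP_Board is the board actor of a board game, giving the position of each player on a given cell.
; On BeginPlay it registers itself with BP_GameMode and caches the length of its CellList, exposed through GetCellNumber.
; GetCellPositionByNumber asks the cell for that player's socket position.
; From a hardcoded index of 21, independent of the cell count, it instead shows WB_Win and pauses the game.
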(event EventBeginPlay
  (bind _asbp_game_mode (Utilities|Casting|CastToBP_GameMode (Game|GetGameMode)))
  (bind _output_get (Variables|Default|SetAs%20BP%20Game%20Mode _asbp_game_mode))
  (bind _output_get_2 (Variables|/Game/BP_GameMode.BP_GameMode_C|SetBoard _output_get self))
  ;[1 1 1] Calcul du nombre de casses du tableau
  (Variables|Default|SetCaseNumber (Utilities|Array|Length (Variables|BP_Board_C|GetCellList _output_get_2))))

(event Collision|EventActorBeginOverlap
  (params (OtherActor :type Actor%20Object%20Reference)))

(event EventTick
  (params (DeltaSeconds :type Float%20%28single-precision%29)))

(fn ConstructionScript)

(fn GetCellPositionbyNumber
  (params (Cell%20Index :type Integer) (Player%20ID :type Integer))
  (bind _returnvalue (Game|GetPlayerController 0))
  ;[1 1 1] Travail perso fonctionnel
  (if (>= Cell%20Index 21)
    (bind _returnvalue_2 (UserInterface|CreateWidget "/Game/WB_Win.WB_Win_C" _returnvalue))
    (UserInterface|Viewport|AddtoViewport _returnvalue_2 0)
    (Variables|/Script/Engine.PlayerController|SetbShowMouseCursor _returnvalue true)
    (Game|SetGamePaused true)
    (else
      (bind _newparam1 (Default|GetSocketPosbyPlayerID (Utilities|Array|Get(acopy) (Variables|Default|GetCellList) Cell%20Index) Player%20ID))
      (return _newparam1))))

(fn GetCellNumber
  (return (Variables|Default|GetCaseNumber)))