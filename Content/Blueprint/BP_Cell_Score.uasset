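; BP_Cell_Score is a cell Blueprint that awards points to a player when its action runs.
; Action calls the parent version, then rewrites that player's entry in the game instance's PlayerList with a higher score, keeping ID and cell number.
; It then shows a points message widget and plays a UI sound.
; The event graph holds only disabled stubs, and the cell-number lookup result goes unused.
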(event EventBeginPlay
  (|CallParentFunction) ; This node is disabled and will not be called.\nDrag off pins to build functionality.
)

(event Collision|EventActorBeginOverlap
  (params (OtherActor :type Actor%20Object%20Reference))
  (|CallParentFunction OtherActor) ; This node is disabled and will not be called.\nDrag off pins to build functionality.
)

(event EventTick
  (params (DeltaSeconds :type Float%20%28single-precision%29))
  (|CallParentFunction DeltaSeconds) ; This node is disabled and will not be called.\nDrag off pins to build functionality.
)

(fn ConstructionScript
  (|CallParentFunction))

(fn Action
  (params (PlayerID :type Integer))
  (bind _as_bp_game_instance (Variables|Default|GetAs%20BP%20Game%20Instance))
  (bind _playerlist (Variables|/Game/BP_GameInstance.BP_GameInstance_C|GetPlayerList _as_bp_game_instance))
  (bind _output (Utilities|Array|Get(acopy) _playerlist PlayerID))
  (bind (_playerid _score _cellnumber) (Utilities|Struct|BreakS_PlayerData _output))
  (|CallParentFunction PlayerID)
  (Default|GetPlayerCellNumberbyPlayerID _as_bp_game_instance PlayerID)
  (Utilities|Array|SetArrayElem (Variables|/Game/BP_GameInstance.BP_GameInstance_C|GetPlayerList _as_bp_game_instance) PlayerID (Utilities|Struct|MakeS_PlayerData _playerid (+ _score 2) _cellnumber))
  (bind _returnvalue (UserInterface|CreateWidget "/Game/Blueprint/Widget/WB_MessagePoints.WB_MessagePoints_C"))
  (UserInterface|Viewport|AddtoViewport _returnvalue 0)
  (Audio|PlaySound2D "/Engine/VREditor/Sounds/UI/Floating_UI_Close-002.Floating_UI_Close-002" 1.0 1.0 0.0 0 0))