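; BP_Window is a clickable tile in the Memory minigame that flips over to show or hide a colored face.
; The construction script sets the Verso material from its Color value.
; An actor click while clickable calls ToggleWindow, which flips the root's roll and IsClickable, then notifies BP_GameModeMemory after a short delay.
; The game mode reference is cached in the separate Verso OnClicked event.
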(event OnClicked(Verso)
  (params (TouchedComponent :type Primitive%20Component%20Object%20Reference) (ButtonPressed :type Key%20Structure :default "None"))
  (bind _asbp_game_mode_memory (Utilities|Casting|CastToBP_GameModeMemory (Game|GetGameMode)))
  (Variables|Default|SetRef%20GM%20Memory _asbp_game_mode_memory))

(event MouseInput|EventActorOnClicked
  (params (ButtonPressed :type Key%20Structure :default "None"))
  (if (Variables|Default|GetIsClickable)
    (CallFunction|ToggleWindow)
    (Utilities|FlowControl|Delay 0.5)
    (Default|OnWindowClick (Variables|Default|GetRef%20GM%20Memory) self)))

(fn ConstructionScript
  (CallFunction|ChangeWindowColor))

(fn ToggleWindow
  (bind _defaultsceneroot (Variables|Default|GetDefaultSceneRoot))
  (Variables|Default|SetIsClickable (not (Variables|Default|GetIsClickable)))
  (if (== (.roll (Transformation|GetWorldRotation (Variables|Default|GetDefaultSceneRoot))) 0.0)
    (Transformation|SetRelativeRotation _defaultsceneroot (Math|Rotator|MakeRotator 1.8e+02 0.0 0.0) false false)
    (else
      (Transformation|SetRelativeRotation _defaultsceneroot (Math|Rotator|MakeRotator 0.0 0.0 0.0) false false))))

(fn ChangeWindowColor
  (bind _verso (Variables|Default|GetVerso))
  (switch Utilities|FlowControl|Switch|SwitchonE_WindowColor (Variables|Default|GetColor)
    (:NewEnumerator0
      (Rendering|Material|SetMaterial _verso 0 "/Game/Blueprint/Memory/Material/MI_Yellow.MI_Yellow"))
    (:NewEnumerator1
      (Rendering|Material|SetMaterial _verso 0 "/Game/Blueprint/Memory/Material/MI_Red.MI_Red"))
    (:NewEnumerator2
      (Rendering|Material|SetMaterial _verso 0 "/Game/Blueprint/Memory/Material/MI_Blue.MI_Blue"))
    (:NewEnumerator3
      (Rendering|Material|SetMaterial _verso 0 "/Game/Blueprint/Memory/Material/MI_Green.MI_Green"))))