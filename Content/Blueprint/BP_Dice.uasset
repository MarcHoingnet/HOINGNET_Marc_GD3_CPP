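; BP_Dice is a dice Blueprint that rolls a configurable number of dice when play begins.
; RollDice resets DiceResult, adds a random value from 1 to DiceType for each of DiceNumber dice, and prints the running total after each roll.
; EndGame is a stub with an always-true branch that does nothing.
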(event EventBeginPlay
  (CallFunction|RollDice))

(fn ConstructionScript)

(fn RollDice
  (Variables|Default|SetDiceResult 0)
  (for _index (range 1 (Variables|Default|GetDiceNumber))
    (bind _output_get (Variables|Default|SetDiceResult (+ (Variables|Default|GetDiceResult) (Math|Random|RandomIntegerinRange 1 (Variables|Default|GetDiceType)))))
    (Development|PrintString (Utilities|String|ToString(Integer) _output_get))))

(fn EndGame
  (if true
    _))