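; Game mode for a two-player dice board game that creates the main widget, both pawns and the die.
; RollDiceAndMove rolls for the current player, clamps the destination to the last board cell, moves the pawn and alternates turns.
; Player cell numbers are stored in the game instance and restore pawn positions at BeginPlay.
; A looping timer polls the pawn's CanDoAction flag to trigger the destination cell's Action on arrival.
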(event Custom|WaitAndAction
  (params (PlayerID :type Integer) (CellDestination :type Integer))
  ;[1 1 1] Vérifier que le joueur atteint la case avant que l'action se lance
  (bind _returnvalue (Utilities|Time|SetTimerbyEvent (delegate Custom|CheckIsArrived) 0.2 true)))

(event Custom|CheckIsArrived
  ;[1 1 1] Vérifier que le joueur atteint la case avant que l'action se lance
  (if (Variables|/Game/Animations/BP_Perso.BP_Perso_C|GetCanDoAction (Utilities|Array|Get(acopy) (Variables|Default|GetPionPlayer) (stale Custom|WaitAndAction PlayerID)))
    (Variables|/Game/Animations/BP_Perso.BP_Perso_C|SetCanDoAction (Utilities|Array|Get(acopy) (Variables|Default|GetPionPlayer) (stale Custom|WaitAndAction PlayerID)) false)
    (Utilities|Time|ClearandInvalidateTimerbyHandle (stale Custom|WaitAndAction _returnvalue))
    (Default|Action (Utilities|Array|Get(acopy) (Variables|/Game/Blueprint/BP_Board.BP_Board_C|GetCellList (Variables|Default|GetBoard)) (stale Custom|WaitAndAction CellDestination)) (stale Custom|WaitAndAction PlayerID))))

(event EventBeginPlay
  ;[1 1 1] widget main
  (bind _returnvalue (UserInterface|CreateWidget "/Game/Blueprint/Collectible/Widget/WB_MainWidget.WB_MainWidget_C"))
  (UserInterface|Viewport|AddtoViewport _returnvalue 0)
  (Variables|Default|SetWidgetRef _returnvalue)
  (bind _asbp_game_instance (Utilities|Casting|CastToBP_GameInstance (Game|GetGameInstance)))
  (bind _output_get (Variables|Default|SetAs%20BP%20Game%20Instance _asbp_game_instance))
  (Utilities|FlowControl|Delay 0.2)
  (for _index (range 0 1)
    ;[1 1 1] Apparition du pion
    (bind _playercellnumber (Default|GetPlayerCellNumberbyPlayerID _output_get _index))
    (bind _cell_location (Default|GetCellPositionbyNumber (Variables|Default|GetBoard) _playercellnumber _index))
    (bind _returnvalue_2 (Game|SpawnActorfromClass "/Game/Animations/BP_Perso.BP_Perso_C" (Math|Conversions|ToTransform(Vector) _cell_location) "AlwaysSpawn" "MultiplyWithRoot" 0 0))
    (Utilities|Array|SetArrayElem (Variables|Default|GetPionPlayer) _index _returnvalue_2 true))
  ;[1 1 1] Spawn dice
  (bind _returnvalue_3 (Game|SpawnActorfromClass "/Game/Blueprint/BP_Dice.BP_Dice_C" (Math|Transform|MakeTransform "0, 0, 0") "Undefined" "MultiplyWithRoot" 0 0))
  (Variables|Default|SetDice _returnvalue_3))

(fn ConstructionScript)

(fn RollDiceandMove
  ;[1 1 1] MAJ score + joueur
  (Default|SetScoreTextbyID (Variables|Default|GetWidgetRef) (Variables|Default|GetActualPlayerID))
  ;[1 1 1] lancement du dé
  (Default|RollDice (Variables|Default|GetDice))
  (Audio|PlaySound2D "/Game/SoundDesign/SFX/SW_LancerDe.SW_LancerDe" 1.0 1.0 0.0 0 0)
  ;[1 1 1] Calculer la case de destination
  (bind _playercellnumber (Default|GetPlayerCellNumberbyPlayerID (Variables|Default|GetAs%20BP%20Game%20Instance) (Variables|Default|GetActualPlayerID)))
  (bind _casenumber (Default|GetCellNumber (Variables|Default|GetBoard)))
  (if (> (+ _playercellnumber (Variables|/Game/Blueprint/BP_Dice.BP_Dice_C|GetDiceResult (Variables|Default|GetDice))) (- _casenumber 1))
    (LocalVariables|SetTempCellDestination (- _casenumber 1))
    (else
      (LocalVariables|SetTempCellDestination (+ _playercellnumber (Variables|/Game/Blueprint/BP_Dice.BP_Dice_C|GetDiceResult (Variables|Default|GetDice))))))
  (CallFunction|MovePawn (LocalVariables|GetTempCellDestination) (Variables|Default|GetActualPlayerID))
  ;[1 1 1] Changement de joueur
  (Variables|Default|SetActualPlayerID (Math|Integer|%(Integer) (+ (Variables|Default|GetActualPlayerID) 1) 2)))

(fn MovePawn
  (params (CellDestination :type Integer) (PlayerID :type Integer))
  ;[1 1 1] Sauvegarde le nouveau numéro de case du joueur
  (Default|SetPlayerCellNumberbyPlayerID (Variables|Default|GetAs%20BP%20Game%20Instance) PlayerID CellDestination)
  ;[1 1 1] Détermine la position finale dans l'espace 3D
  (bind _cell_location (Default|GetCellPositionbyNumber (Variables|Default|GetBoard) CellDestination PlayerID))
  ;[1 1 1] Déplacement du pion
  (Default|MovetoNewCell (Utilities|Array|Get(acopy) (Variables|Default|GetPionPlayer) PlayerID) _cell_location)
  (CallFunction|WaitandAction PlayerID CellDestination))